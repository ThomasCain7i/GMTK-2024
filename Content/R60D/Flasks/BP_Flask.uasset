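; BP_Flask is a configurable flask prop that builds its look in the construction script and has no runtime logic.
; FlaskType selects the meshes from Flasks for the flask, its ShadowCaster duplicate and an optional holder, which is destroyed when unused.
; With Useliquid on, the liquid mesh fills two layers: one with a dynamic material tinted by Color, the other with the M_Bubbler bubble material.
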(event EventBeginPlay)

(event Collision|EventActorBeginOverlap
  (params (OtherActor :type Actor%20Object%20Reference)))

(event EventTick
  (params (DeltaSeconds :type Float%20%28single-precision%29)))

(fn ConstructionScript
  (bind _flasks (Variables|Default|GetFlasks))
  (bind _flasktype (Variables|Default|GetFlaskType))
  (bind _output (Utilities|Array|Get(acopy) _flasks _flasktype))
  (bind (_flask _liquid _holder) (Utilities|Struct|BreakS_Flask _output))
  (if (Variables|Default|GetUseHolder)
    (Components|StaticMesh|SetStaticMesh (Variables|Default|GetHolder) _holder)
    (else
      (Components|DestroyComponent (Variables|Default|GetHolder))))
  (Components|StaticMesh|SetStaticMesh (Variables|Default|GetFlask) _flask)
  (Components|StaticMesh|SetStaticMesh (Variables|Default|GetShadowCaster) _flask)
  (if (Variables|Default|GetUseliquid)
    (Components|StaticMesh|SetStaticMesh (Variables|Default|GetLiquidLayer) _liquid)
    (Rendering|Material|SetMaterial (Variables|Default|GetLiquidLayer) 0 (Variables|Default|GetLiquid))
    (bind _returnvalue (Rendering|Material|CreateDynamicMaterialInstance (Variables|Default|GetLiquidLayer) 0 (Variables|Default|GetLiquid) "None" :!class /Script/Engine.PrimitiveComponent))
    (Rendering|Material|SetVectorParameterValue _returnvalue "Color" (Variables|Default|GetColor) :!class /Script/Engine.MaterialInstanceDynamic)
    (Components|StaticMesh|SetStaticMesh (Variables|Default|GetBubbleLayer) _liquid)
    (Rendering|Material|SetMaterial (Variables|Default|GetBubbleLayer) 0 "/Game/R60D/Flasks/M_Bubbler.M_Bubbler")))