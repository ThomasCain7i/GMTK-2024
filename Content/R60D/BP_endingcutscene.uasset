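; Ending cutscene trigger actor that plays the final sequence and returns the game to the main menu.
; The referenced skeletal mesh actor is hidden on BeginPlay.
; When the third-person character first overlaps the box, it reveals and animates that mesh, destroys the player character and plays the level sequence.
; When the sequence finishes, it opens the MainMenu level.
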(event OnComponentBeginOverlap(Box)
  (params (OverlappedComponent :type Primitive%20Component%20Object%20Reference) (OtherActor :type Actor%20Object%20Reference) (OtherComp :type Primitive%20Component%20Object%20Reference) (OtherBodyIndex :type Integer) (bFromSweep :type Boolean) (SweepResult :type Hit%20Result%20Structure%20%28by%20ref%29))
  (bind _cutscene (Variables|Default|GetCutscene))
  (bind _skeletal (Variables|Default|GetSkeletal))
  (bind _sequenceplayer (Variables|/Script/LevelSequence.LevelSequenceActor|GetSequencePlayer _cutscene))
  (bind _asbp_third_person_character (Utilities|Casting|CastToBP_ThirdPersonCharacter OtherActor))
  (Utilities|FlowControl|DoOnce false
    (:Completed
      (Audio|Components|Audio|Play (Variables|/Script/Engine.SkeletalMeshActor|GetSkeletalMeshComponent _skeletal) false)
      (Rendering|SetVisibility (Variables|/Script/Engine.Actor|GetRootComponent _skeletal) true false)
      (Actor|DestroyActor _asbp_third_person_character)
      (Sequencer|Player|Play _sequenceplayer :!class /Script/MovieScene.MovieSceneSequencePlayer)
      (EventDispatchers|BindEventtoOnFinished _sequenceplayer (delegate Custom|eND)))))

(event Custom|eND
  (Game|OpenLevel(byName) "MainMenu"))

(event Collision|EventActorBeginOverlap
  (params (OtherActor :type Actor%20Object%20Reference)))

(event EventTick
  (params (DeltaSeconds :type Float%20%28single-precision%29)))

(event EventBeginPlay
  (Rendering|SetVisibility (Variables|/Script/Engine.Actor|GetRootComponent (Variables|Default|GetSkeletal)) false false))

(fn ConstructionScript)