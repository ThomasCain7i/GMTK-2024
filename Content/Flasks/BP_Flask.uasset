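; BP_Flask is a configurable flask prop that shows a vessel with colored liquid and bubbles inside.
; Its construction script uses FlaskType to pick the vessel and liquid meshes from the Flasks collection, with ShadowCaster duplicating the vessel mesh.
; LiquidLayer gets a dynamic material instance tinted by Color, while BubbleLayer reuses the liquid mesh with the M_Bubbler material.
; The event graph has no active logic.
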(event EventBeginPlay)

(event Collision|EventActorBeginOverlap
  (params (OtherActor :type Actor%20Object%20Reference)))

(event EventTick
  (params (DeltaSeconds :type Float%20%28single-precision%29)))

(fn ConstructionScript
  (bind _flasks (Variables|Default|GetFlasks))
  (bind _liquidlayer (Variables|Default|GetLiquidLayer))
  (bind _bubblelayer (Variables|Default|GetBubbleLayer))
  (bind _flasktype (Variables|Default|GetFlaskType))
  (bind _liquid (Variables|Default|GetLiquid))
  (bind _output (Utilities|Array|Get(acopy) _flasks _flasktype))
  (bind (_flask _liquid_2) (Utilities|Struct|BreakS_Flask _output))
  (Components|StaticMesh|SetStaticMesh (Variables|Default|GetFlask) _flask)
  (Components|StaticMesh|SetStaticMesh (Variables|Default|GetShadowCaster) _flask)
  (Components|StaticMesh|SetStaticMesh _liquidlayer _liquid_2)
  (Rendering|Material|SetMaterial _liquidlayer 0 _liquid)
  (bind _returnvalue (Rendering|Material|CreateDynamicMaterialInstance _liquidlayer 0 _liquid "None" :!class /Script/Engine.PrimitiveComponent))
  (Rendering|Material|SetVectorParameterValue _returnvalue "Color" (Variables|Default|GetColor) :!class /Script/Engine.MaterialInstanceDynamic)
  (Components|StaticMesh|SetStaticMesh _bubblelayer _liquid_2)
  (Rendering|Material|SetMaterial _bubblelayer 0 "/Game/Flasks/M_Bubbler.M_Bubbler"))