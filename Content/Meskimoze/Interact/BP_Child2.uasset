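; BP_Child2 is a conveyor-style interactable that pushes any actor overlapping its Box along the forward direction of its Arrow.
; Each Tick it loops through the overlapping actors and scales the push by Speed and delta time.
; BP_Child actors receive a physics impulse on their StaticMesh, while all other actors are moved by a non-swept world offset.
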(event EventTick
  (params (DeltaSeconds :type Float%20%28single-precision%29))
  (bind _speed (Variables|Default|GetSpeed))
  (bind _arrow (Variables|Default|GetArrow))
  (bind _returnvalue (Transformation|GetWorldRotation _arrow))
  (bind _returnvalue_2 (* DeltaSeconds _speed))
  (bind _returnvalue_3 (Math|Vector|GetForwardVector _returnvalue))
  (bind _returnvalue_4 (* _returnvalue_2 _returnvalue_3))
  (for _array_element (Collision|GetOverlappingActors (Variables|Default|GetBox) 0 :!class /Script/Engine.PrimitiveComponent)
    (bind _asbp_child (Utilities|Casting|CastToBP_Child _array_element)
      (:then
        (Physics|AddImpulse (Variables|/Game/Meskimoze/Interact/BP_Child.BP_Child_C|GetStaticMesh _asbp_child) (* _returnvalue_4 1e+03) "None" false))
      (:CastFailed
        (Transformation|AddActorWorldOffset _array_element _returnvalue_4)))))

(fn ConstructionScript
  (|CallParentFunction))