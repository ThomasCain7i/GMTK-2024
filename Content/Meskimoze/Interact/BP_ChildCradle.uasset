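; BP_ChildCradle is an interactable cradle whose animation and sound follow a Speed value.
; Each Tick rounds Speed up to steps of 1/Increment and uses the result as the skeletal mesh play rate.
; The absolute stepped value drives the audio pitch, and the sound is muted when that value is near zero.
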(event EventBeginPlay)

(event Collision|EventActorBeginOverlap
  (params (OtherActor :type Actor%20Object%20Reference)))

(event EventTick
  (params (DeltaSeconds :type Float%20%28single-precision%29))
  (bind _increment (Variables|Default|GetIncrement))
  (bind _speed (Variables|Default|GetSpeed))
  (bind _audio_0 (Variables|Default|GetAudio_0))
  (bind _returnvalue (* _speed _increment))
  (bind _returnvalue_2 (Math|Float|Ceil _returnvalue))
  (bind _returnvalue_3 (/ _returnvalue_2 _increment))
  (Components|Timeline|SetPlayRate (Variables|Default|GetSkeletalMesh) _returnvalue_3)
  (Audio|Components|Audio|SetPitchMultiplier _audio_0 (Math|Float|Absolute(Float) _returnvalue_3))
  (Audio|Components|Audio|SetVolumeMultiplier _audio_0 (Math|Float|SelectFloat 0.0 1.0 (Math|Float|InRange(Float) _returnvalue_3 -0.1 0.1)) :!class /Script/Engine.AudioComponent))

(fn ConstructionScript
  (|CallParentFunction))