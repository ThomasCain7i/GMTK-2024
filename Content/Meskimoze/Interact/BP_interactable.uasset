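; Base interactable that the player can highlight and either resize or speed up and slow down.
; Highlight applies an overlay material to all meshes and clears it on a one-second timer.
; OnInteract runs per-axis or uniform scale macros on BP_Child's mesh via a self-cast, playing a non-overlapping voice line at size limits.
; Non-scalable objects adjust a bounded Speed value instead, with both steps normalized by delta time.
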(event Custom|Remove
  (for _array_element (Actor|GetComponentsByClass "/Script/Engine.MeshComponent")
    (Rendering|Material|SetOverlayMaterial _array_element 0 :!class /Script/Engine.MeshComponent))
  (Variables|Default|SetReady true))

(event EventHighlight
  (Utilities|Time|SetTimerbyEvent (delegate Custom|Remove) 1.0)
  (if (Variables|Default|GetReady)
    (Variables|Default|SetReady false)
    (for _array_element (Actor|GetComponentsByClass "/Script/Engine.MeshComponent")
      (Rendering|Material|SetOverlayMaterial _array_element (Variables|Default|GetMaterial) :!class /Script/Engine.MeshComponent))))

(event EventBeginPlay)

(event EventOnInteract
  (params (Scalable%20? :type Boolean) (Mode :type Integer) (ScalingUp? :type Boolean))
  (if Scalable%20?
    (if ScalingUp?
      (switch int Mode
        (:0
          (|XAxisUP
            (:Completed
              _)))
        (:1
          (|YAxisUP
            (:Completed
              _)))
        (:2
          (|ZAxisUP
            (:Completed
              _)))
        (:3
          (|AllAxisUP
            (:Completed
              _))))
      (if (Utilities|IsValid (Variables|Default|GetAudioPlaying))
        (if (not (Audio|Components|Audio|IsPlaying (Variables|Default|GetAudioPlaying)))
          (bind _returnvalue (Audio|SpawnSound2D "/Game/SFX/doc_line_too_big.doc_line_too_big" 0.5 1.0 0.0 0 :!label _label))
          (Variables|Default|SetAudioPlaying _returnvalue))
        (else
          (goto _label)))
      (else
        (switch int Mode
          (:0
            (|XAxisDown
              (:Completed
                _)))
          (:1
            (|YAxisDown
              (:Completed
                _)))
          (:2
            (|ZAxisDown
              (:Completed
                _)))
          (:3
            (|AllAxisDown
              (:Completed
                _))))
        (if (Utilities|IsValid (Variables|Default|GetAudioPlaying))
          (if (not (Audio|Components|Audio|IsPlaying (Variables|Default|GetAudioPlaying)))
            (bind _returnvalue_2 (Audio|SpawnSound2D "/Game/SFX/doc_line_too_small.doc_line_too_small" 0.5 1.0 0.0 0 :!label _label_2))
            (Variables|Default|SetAudioPlaying _returnvalue_2))
          (else
            (goto _label_2)))))
    (else
      (|SpeedUpDown ScalingUp?))))

(fn ConstructionScript)